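; BP_Switch is a switch actor that animates between on and off and drives the devices connected to it.
; It can be set to an explicit state, acting only on a change, or toggled with a flip-flop event.
; BeginPlay and both events play the matching animation and push the state to each DeviceConnected entry through the BPI_Switchable_Lamps interface, passing itself as the source actor.
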(event `/Game/Blueprints/Interfaces/BPI_Switchable.Switch_WithBool`
  (params (Actor :type "Actor Object Reference") (Owner :type "Pawn Object Reference") (`On?` :type Boolean))
  (bind _switch (`self.Switch`))
  (if (!= `On?` (`self.On?`))
    (bind _output_get (set `self.On?` `On?`))
    (if _output_get
      (`SkeletalMeshComponent.PlayAnimation` _switch "/Game/Core/Mesh/Switch/AS_Switch_To_On.AS_Switch_To_On" false)
      (else
        (`SkeletalMeshComponent.PlayAnimation` _switch "/Game/Core/Mesh/Switch/AS_Switch_To_OFF.AS_Switch_To_OFF" false)))
    (`self.Update_Device` Owner)))

(event `/Game/Blueprints/Interfaces/BPI_Switchable.Switch_FlipFlop`
  (params (Actor :type "Actor Object Reference") (Owner :type "Pawn Object Reference"))
  (bind _switch (`self.Switch`))
  (bind _output_get (set `self.On?` (not (`self.On?`))))
  (if _output_get
    (`SkeletalMeshComponent.PlayAnimation` _switch "/Game/Core/Mesh/Switch/AS_Switch_To_On.AS_Switch_To_On" false)
    (else
      (`SkeletalMeshComponent.PlayAnimation` _switch "/Game/Core/Mesh/Switch/AS_Switch_To_OFF.AS_Switch_To_OFF" false)))
  (`self.Update_Device` Owner))

(event `self.ReceiveBeginPlay`
  (bind _on_ (`self.On?`))
  (bind _switch (`self.Switch`))
  (`|ExecutionSequence`
    (:`then_0`
      (if _on_
        (`SkeletalMeshComponent.PlayAnimation` _switch "/Game/Core/Mesh/Switch/AS_Switch_To_On.AS_Switch_To_On" false)
        (else
          (`SkeletalMeshComponent.PlayAnimation` _switch "/Game/Core/Mesh/Switch/AS_Switch_To_OFF.AS_Switch_To_OFF" false)))
      (for _array_element (`self.Device_Connected`)
        (bind _asbpi_switchable_lamps (cast `/Game/Blueprints/Interfaces/BPI_Switchable_Lamps` _array_element))
        (`/Game/Blueprints/Interfaces/BPI_Switchable_Lamps.Switch_WithBool` _asbpi_switchable_lamps self null _on_)))))

(event `Update_Device`
  (params (Owner :type "Pawn Object Reference"))
  (for _array_element (`self.Device_Connected`)
    (bind _asbpi_switchable_lamps (cast `/Game/Blueprints/Interfaces/BPI_Switchable_Lamps` _array_element))
    (`/Game/Blueprints/Interfaces/BPI_Switchable_Lamps.Switch_WithBool` _asbpi_switchable_lamps self null (`self.On?`))))

(fn `UserConstructionScript`)