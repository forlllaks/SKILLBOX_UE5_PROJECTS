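; Player controller (TPC) that drives the possessed character's movement and camera look and handles interaction with nearby switchable objects.
; BeginPlay caches the character, adds the Enhanced Input mapping context, creates the game HUD and starts a looping timer.
; The timer uses a sphere overlap to maintain a list of nearby BPI_Switchable actors.
; Select input cycles the list index, and Interact calls SwitchFlipFlop on that entry, then OnInteracting.
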(event `Update_InteractList`
  (bind _interactlist (`self.InteractList`))
  ;[1 0.4947 0.6153] Каждое определённое время проверяю на наличие возможности с чем то интерактировать
  (bind _outactors (`KismetSystemLibrary.SphereOverlapActors` (`self.K2_GetActorLocation` (`self.CharacterControlled`)) (`self.Interact_Radius`) (`|MakeArray` "ObjectTypeQuery3" "ObjectTypeQuery2" "ObjectTypeQuery1" :!type "EObjectTypeQuery Enum") "/Script/Engine.Actor" (`|MakeArray` (`self.CharacterControlled`) :!type "Actor Object Reference")))
  (for _array_element _interactlist
    (if (== (`KismetArrayLibrary.Array_Find` _outactors _array_element) -1)
      (`KismetArrayLibrary.Array_RemoveItem` _interactlist _array_element)))
  (for _array_element_2 _outactors
    (cast `/Game/Blueprints/Interfaces/BPI_Switchable` _array_element_2)
    (`KismetArrayLibrary.Array_AddUnique` _interactlist _array_element_2)))

(event `self.ReceiveBeginPlay`
  (`|ExecutionSequence`
    (:`then_0`
      (set `self.Controller` self)
      (bind _ascharacter (cast `Character` (`GameplayStatics.GetPlayerPawn` 0)))
      (set `self.CharacterControlled` _ascharacter)
      (set `self.MovementComponent` (`Pawn.GetMovementComponent` _ascharacter))
      (`EnhancedInputSubsystemInterface.AddMappingContext` (pcsubsystem `EnhancedInputLocalPlayerSubsystem` self) "/Game/Core/Inputs/Mapping/IM_GameInput_TPC.IM_GameInput_TPC" 0 (struct))
      (bind _returnvalue (`|CreateWidget` "/Game/Core/UI/UI_TPC_Game.UI_TPC_Game_C" self self))
      (`UserWidget.AddToViewport` _returnvalue 0))
    (:`then_1`
      (`KismetSystemLibrary.K2_SetTimerDelegate` (delegate `Update_InteractList`) 0.3 true))))

(event `self.ReceiveTick`
  (params (DeltaSeconds :type "Float (single-precision)")))

(event `EnhancedInput|/Game/Core/Inputs/Actions/IA_TPC_InteractSelect`
  (params (ActionValue :type "Float (double-precision)") (ElapsedSeconds :type "Float (double-precision)") (TriggeredSeconds :type "Float (double-precision)") (InputAction :type "InputAction Object Reference" :default "/Game/Core/Inputs/Actions/IA_TPC_InteractSelect.IA_TPC_InteractSelect"))
  (bind _returnvalue (+ (`self.Interact_Index`) ActionValue))
  (bind _returnvalue_2 (`KismetMathLibrary.Conv_IntToDouble` (`KismetArrayLibrary.Array_Length` (`self.InteractList`))))
  (bind _returnvalue_3 (- _returnvalue_2 1.0))
  ;[0.8604 1 0.439] Выбираю индекс интеракта
  (:`Triggered`
    (if (>= _returnvalue _returnvalue_2)
      (set `self.Interact_Index` -1))
    (if (== _returnvalue -1.0)
      (set `self.Interact_Index` (`KismetMathLibrary.FTrunc` _returnvalue_3))
      (else
        (set `self.Interact_Index` (`KismetMathLibrary.FTrunc` (`KismetMathLibrary.FClamp` _returnvalue 0.0 _returnvalue_3)))))))

(event `EnhancedInput|/Game/Core/Inputs/Actions/IA_TPC_Interact`
  (params (ActionValue :type Boolean) (ElapsedSeconds :type "Float (double-precision)") (TriggeredSeconds :type "Float (double-precision)") (InputAction :type "InputAction Object Reference" :default "/Game/Core/Inputs/Actions/IA_TPC_Interact.IA_TPC_Interact"))
  ;[1 0.5687 0.2819] Получаю обьект по индексу и вызываю евент
  (:`Completed`
    (bind _asbpi_switchable (cast `/Game/Blueprints/Interfaces/BPI_Switchable` (`|GetArrayItem` (`self.InteractList`) (`self.Interact_Index`))))
    (`/Game/Blueprints/Interfaces/BPI_Switchable.Switch_FlipFlop` _asbpi_switchable null (`self.CharacterControlled`))
    (`self.OnInteracting`)))

(event `EnhancedInput|/Game/Core/Inputs/Actions/IA_TPC_Look`
  (params (ActionValue :type "Vector2D Structure") (ElapsedSeconds :type "Float (double-precision)") (TriggeredSeconds :type "Float (double-precision)") (InputAction :type "InputAction Object Reference" :default "/Game/Core/Inputs/Actions/IA_TPC_Look.IA_TPC_Look"))
  (bind _controller (`self.Controller`))
  (:`Triggered`
    (`self.AddPitchInput` _controller ActionValue_Y)
    (`self.AddYawInput` _controller ActionValue_X)))

(event `EnhancedInput|/Game/Core/Inputs/Actions/IA_TPC_Walk`
  (params (ActionValue :type "Vector2D Structure") (ElapsedSeconds :type "Float (double-precision)") (TriggeredSeconds :type "Float (double-precision)") (InputAction :type "InputAction Object Reference" :default "/Game/Core/Inputs/Actions/IA_TPC_Walk.IA_TPC_Walk"))
  (bind (_returnvalue_roll _returnvalue_pitch _returnvalue_yaw) (`KismetMathLibrary.BreakRotator` (`self.GetControlRotation`)))
  (bind (_returnvalue_roll_2 _returnvalue_pitch_2 _returnvalue_yaw_2) (`KismetMathLibrary.BreakRotator` (`self.GetControlRotation`)))
  (bind _movementcomponent (`self.MovementComponent`))
  (:`Triggered`
    (`PawnMovementComponent.AddInputVector` _movementcomponent (* ActionValue_X (`KismetMathLibrary.GetForwardVector` (`KismetMathLibrary.MakeRotator` 0.0 0.0 _returnvalue_yaw_2))) false)
    (`PawnMovementComponent.AddInputVector` _movementcomponent (* ActionValue_Y (`KismetMathLibrary.GetRightVector` (`KismetMathLibrary.MakeRotator` _returnvalue_roll 0.0 _returnvalue_yaw))) false)))

(fn `UserConstructionScript`)