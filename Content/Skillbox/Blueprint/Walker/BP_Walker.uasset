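; BP_Walker is a pawn that wanders endlessly between random reachable navigation points within a large radius.
; From BeginPlay, WalkToRandomPoint picks a destination and runs AIMoveTo, then calls itself again after a short delay on success or failure.
; Each Tick places Arrow2 just below the destination and, while the pawn moves, turns Arrow1's yaw to follow the FloatingPawnMovement velocity.
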(event `WalkToRandomPoint`
  (bind _output_get (set `self.FinishLocation` (`NavigationSystemV1.K2_GetRandomReachablePointInRadius` (`self.K2_GetActorLocation`) 50000.0 null null)))
  (`|AIMoveTo` self _output_get null
    (:`OnSuccess`
      (`KismetSystemLibrary.Delay` 0.5)
      (`self.WalkToRandomPoint`))
    (:`OnFail`
      (`KismetSystemLibrary.Delay` 0.2)
      (`self.WalkToRandomPoint`))))

(event `self.ReceiveBeginPlay`
  (`self.WalkToRandomPoint`))

(event `self.ReceiveTick`
  (params (DeltaSeconds :type "Float (single-precision)"))
  (bind _returnvalue (`SceneComponent.K2_GetComponentLocation` (`self.Cube`)))
  (bind (_returnvalue_roll _returnvalue_pitch _returnvalue_yaw) (`KismetMathLibrary.BreakRotator` (`KismetMathLibrary.FindLookAtRotation` _returnvalue (- _returnvalue (`MovementComponent.Velocity` (`self.FloatingPawnMovement`))))))
  (`|ExecutionSequence`
    (:`then_0`
      (`SceneComponent.K2_SetWorldLocation` (`self.Arrow2`) (- (`self.FinishLocation`) (0.0 0.0 4.0)) false true))
    (:`then_1`
      (if (not (== (`MovementComponent.Velocity` (`self.FloatingPawnMovement`)) (0.0 0.0 0.0)))
        (`SceneComponent.K2_SetWorldRotation` (`self.Arrow1`) (`KismetMathLibrary.MakeRotator` 180.0 180.0 _returnvalue_yaw) false true)))))

(fn `UserConstructionScript`)